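; BP_SpeechTrigger is a one-shot trigger that shows a tutorial line explaining that fuses restore power to parts of the store.
; On BeginPlay it waits briefly, then hides the speech text through the player character's SpeechBoxRef.
; The first Box overlap passes a DoOnce before the character cast, shows the hardcoded line, then hides it after a delay.
; Any overlapping actor, player or not, uses up that single trigger.
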(event OnComponentBeginOverlap(Box)
  (params (OverlappedComponent :type Primitive%20Component%20Object%20Reference) (OtherActor :type Actor%20Object%20Reference) (OtherComp :type Primitive%20Component%20Object%20Reference) (OtherBodyIndex :type Integer) (bFromSweep :type Boolean) (SweepResult :type Hit%20Result%20Structure%20%28by%20ref%29))
  (Utilities|FlowControl|DoOnce false
    (:Completed
      (bind _asbp_third_person_character (Utilities|Casting|CastToBP_ThirdPersonCharacter OtherActor))
      (Default|UpdateSpeechText (Variables|/Game/ThirdPerson/Blueprints/BP_ThirdPersonCharacter.BP_ThirdPersonCharacter_C|GetSpeechBoxRef _asbp_third_person_character) "This is a Fuse. You need these to restore power to different parts of the store.  ")
      (Utilities|FlowControl|Delay 4.0)
      (Default|HideSpeechText (Variables|/Game/ThirdPerson/Blueprints/BP_ThirdPersonCharacter.BP_ThirdPersonCharacter_C|GetSpeechBoxRef _asbp_third_person_character)))))

(event EventBeginPlay
  (Utilities|FlowControl|Delay 0.2)
  (bind _asbp_third_person_character (Utilities|Casting|CastToBP_ThirdPersonCharacter (Game|GetPlayerCharacter 0)))
  (Default|HideSpeechText (Variables|/Game/ThirdPerson/Blueprints/BP_ThirdPersonCharacter.BP_ThirdPersonCharacter_C|GetSpeechBoxRef _asbp_third_person_character)))

(event EventTick
  (params (DeltaSeconds :type Float%20%28single-precision%29)))

(fn ConstructionScript)