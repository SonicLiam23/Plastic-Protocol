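; BP_Ammo is an ammo pickup that refills the interacting character's equipped weapon when its type matches the box's AmmoBoxType.
; The construction script picks a box or magazine mesh from that type.
; On Interact, it reads the character's equipped weapon, adds one full clip to reserve ammo, sets the last WeaponStats field to false, then destroys itself.
; Its own GetEquippedWeapon function is an empty stub.
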(event EventBeginPlay)

(event Collision|EventActorBeginOverlap
  (params (OtherActor :type Actor%20Object%20Reference)))

(event EventTick
  (params (DeltaSeconds :type Float%20%28single-precision%29)))

(event EventInteract
  (params (CharacterPickingUp :type BP%20Third%20Person%20Character%20Object%20Reference))
  (bind _activeweapon (Default|GetEquippedWeapon CharacterPickingUp))
  (Utilities|IsValid _activeweapon
    (:Is%20Valid
      (if (Utilities|Enum|Equal(Enum) (Variables|Default|GetAmmoBoxType) (Variables|/Game/_Project/Props/Weapons/BP_WeaponMaster.BP_WeaponMaster_C|GetWeaponType _activeweapon))
        (Variables|/Game/_Project/Props/Weapons/BP_WeaponMaster.BP_WeaponMaster_C|SetWeaponStats _activeweapon (Utilities|Struct|MakeS_WeaponData (.currentclip (Variables|/Game/_Project/Props/Weapons/BP_WeaponMaster.BP_WeaponMaster_C|GetWeaponStats _activeweapon)) (.maxclip (Variables|/Game/_Project/Props/Weapons/BP_WeaponMaster.BP_WeaponMaster_C|GetWeaponStats _activeweapon)) (+ (.maxclip (Variables|/Game/_Project/Props/Weapons/BP_WeaponMaster.BP_WeaponMaster_C|GetWeaponStats _activeweapon)) (.reserveammo (Variables|/Game/_Project/Props/Weapons/BP_WeaponMaster.BP_WeaponMaster_C|GetWeaponStats _activeweapon))) (.firerate (Variables|/Game/_Project/Props/Weapons/BP_WeaponMaster.BP_WeaponMaster_C|GetWeaponStats _activeweapon)) false))
        (Actor|DestroyActor)))))

(fn ConstructionScript
  (switch Utilities|FlowControl|Switch|SwitchonEnum_WeaponType (Variables|Default|GetAmmoBoxType)
    (:NewEnumerator1
      (Components|StaticMesh|SetStaticMesh (Variables|Default|GetAmmo) "/Game/Student_Assets/Daniel/Ammo/BoxAmmoBox.BoxAmmoBox"))
    (:NewEnumerator3
      (Components|StaticMesh|SetStaticMesh (Variables|Default|GetAmmo) "/Game/Student_Assets/Daniel/Ammo/MagAmmoBox.MagAmmoBox"))))

(fn GetEquippedWeapon
  (return 0))