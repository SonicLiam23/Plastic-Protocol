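; Electric box terminal that restores power when the third-person character enters its trigger box carrying at least three fuses.
; On success it removes the objective marker widget and, once, updates the objective, toggles every RectLight's visibility, shows its fuse meshes and hides a static mesh.
; The success path only runs if a marker widget exists.
; With too few fuses, the player's speech box shows a hint for a few seconds.
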(event OnComponentBeginOverlap(Box)
  (params (OverlappedComponent :type Primitive%20Component%20Object%20Reference) (OtherActor :type Actor%20Object%20Reference) (OtherComp :type Primitive%20Component%20Object%20Reference) (OtherBodyIndex :type Integer) (bFromSweep :type Boolean) (SweepResult :type Hit%20Result%20Structure%20%28by%20ref%29))
  (bind _asbp_third_person_character (Utilities|Casting|CastToBP_ThirdPersonCharacter OtherActor))
  (if (>= (Variables|/Game/ThirdPerson/Blueprints/BP_ThirdPersonCharacter.BP_ThirdPersonCharacter_C|GetFuseCount _asbp_third_person_character) 3)
    (bind _foundwidgets (Widget|GetAllWidgetsOfClass "/Game/GW_ProjFiles/WBP_ObjectiveMarker.WBP_ObjectiveMarker_C" true))
    (Utilities|IsValid (Utilities|Array|Get(acopy) _foundwidgets)
      (:Is%20Valid
        (Widget|RemovefromParent (Utilities|Array|Get(acopy) _foundwidgets))
        (Utilities|FlowControl|DoOnce false
          (:Completed
            (Default|UpdateObjective _asbp_third_person_character "Power Restored!" 1 1)
            (bind _outactors (Actor|GetAllActorsOfClass "/Script/Engine.RectLight"))
            (for _array_element _outactors
              (Rendering|ToggleVisibility (Variables|/Script/Engine.Light|GetLightComponent _array_element) false)
              (Rendering|SetVisibility (Variables|Default|GetFuse4) true false)
              (Actor|GetAllActorsOfClass "/Game/GW_ProjFiles/BP_FloorLighting.BP_FloorLighting_C")
              (Rendering|SetVisibility (Variables|Default|GetStaticMesh) false false))))))
    (else
      (Default|UpdateSpeechText (Variables|/Game/ThirdPerson/Blueprints/BP_ThirdPersonCharacter.BP_ThirdPersonCharacter_C|GetSpeech%20Box%20Ref _asbp_third_person_character) "You don't have enough fuses to turn the power on at this terminal. Find some around the Store! ")
      (Utilities|FlowControl|Delay 4.0)
      (Default|HideSpeechText (Variables|/Game/ThirdPerson/Blueprints/BP_ThirdPersonCharacter.BP_ThirdPersonCharacter_C|GetSpeech%20Box%20Ref _asbp_third_person_character)))))

(event EventBeginPlay)

(event Collision|EventActorBeginOverlap
  (params (OtherActor :type Actor%20Object%20Reference)))

(event EventTick
  (params (DeltaSeconds :type Float%20%28single-precision%29)))

(fn ConstructionScript)