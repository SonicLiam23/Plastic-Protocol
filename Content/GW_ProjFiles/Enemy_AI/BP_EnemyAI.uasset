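; BP_EnemyAI is an AI-controlled enemy character that fires projectiles and dies when its health runs out.
; StartFiring and StopFiring toggle a looping timer that spawns a projectile with muzzle effect and sound.
; On death from its Health component it stops firing, unpossesses, disables collision, plays a death montage and destroys itself after a short delay.
; A helper function sets its max walk speed.
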(event OnDeath(Health)
  (if (<= (Variables|/Script/ToySoldiers.HealthComponent|GetCurrentHealth (Variables|Default|GetHealth)) 0.0)
    (Utilities|FlowControl|DoOnce false
      (:Completed
        (CallFunction|StopFiring)
        (Pawn|UnPossess (Pawn|GetController))
        (Collision|SetCollisionEnabled (Variables|Collision|GetCapsuleComponent) "NoCollision")
        (Animation|PlayAnimMontage "/Game/GW_ProjFiles/EnemyAnims/Anims/Death/MM_Death_Front_01_Montage.MM_Death_Front_01_Montage" 1.0 "None")
        (Utilities|FlowControl|Delay 1.0)
        (Actor|DestroyActor)))))

(event Custom|Fire%20Weapon
  (bind _mesh (Variables|Character|GetMesh))
  (bind _returnvalue (Transformation|GetSocketLocation _mesh "Muzzle"))
  (Class|ProjectileSpawner|SpawnProjectile (Variables|Default|GetBP_ProjectileSpawner))
  (Effects|SpawnEmitteratLocation 0 _returnvalue)
  (Audio|PlaySoundatLocation 0 _returnvalue "0, 0, 0" 1.0 1.0 0.0 0 0 0 0))

(event Custom|Start%20Firing
  (bind _returnvalue (Utilities|Time|SetTimerbyEvent (delegate Custom|Fire%20Weapon) 0.8 true))
  (Variables|Default|SetFireTimerHandle _returnvalue))

(event Custom|Stop%20Firing
  (Utilities|Time|ClearandInvalidateTimerbyHandle (Variables|Default|GetFireTimerHandle)))

(event EventBeginPlay)

(event Collision|EventActorBeginOverlap
  (params (OtherActor :type Actor%20Object%20Reference)))

(event EventTick
  (params (DeltaSeconds :type Float%20%28single-precision%29)))

(fn ConstructionScript)

(fn SetMaxWalkspeed
  (params (Speed :type Float%20%28double-precision%29))
  (Variables|/Script/Engine.CharacterMovementComponent|SetMaxWalkSpeed (Variables|Character|GetCharacterMovement) Speed))