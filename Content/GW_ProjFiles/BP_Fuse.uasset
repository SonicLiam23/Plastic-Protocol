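; BP_Fuse is a collectible fuse pickup in a gather-and-repair objective.
; On any sphere overlap, without checking what overlapped, it increments the player character's FuseCount, updates the objective progress and destroys itself.
; When the count reaches three, it switches the objective to finding the Electric Box and adds a WBP_ObjectiveMarker widget targeting the BP_ElectricBox actor.
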(event OnComponentBeginOverlap(Sphere)
  (params (OverlappedComponent :type Primitive%20Component%20Object%20Reference) (OtherActor :type Actor%20Object%20Reference) (OtherComp :type Primitive%20Component%20Object%20Reference) (OtherBodyIndex :type Integer) (bFromSweep :type Boolean) (SweepResult :type Hit%20Result%20Structure%20%28by%20ref%29))
  (bind _asbp_third_person_character (Utilities|Casting|CastToBP_ThirdPersonCharacter (Game|GetPlayerCharacter 0)))
  (bind _output_get (Variables|/Game/ThirdPerson/Blueprints/BP_ThirdPersonCharacter.BP_ThirdPersonCharacter_C|SetFuseCount _asbp_third_person_character (+ (Variables|/Game/ThirdPerson/Blueprints/BP_ThirdPersonCharacter.BP_ThirdPersonCharacter_C|GetFuseCount _asbp_third_person_character) 1)))
  (if (== _output_get 3)
    (Default|UpdateObjective _asbp_third_person_character "Find the Electric Box" 0 1)
    (bind _returnvalue (Actor|GetActorOfClass "/Game/GW_ProjFiles/BP_ElectricBox.BP_ElectricBox_C"))
    (bind _returnvalue_2 (UserInterface|CreateWidget "/Game/GW_ProjFiles/WBP_ObjectiveMarker.WBP_ObjectiveMarker_C" 0 _returnvalue))
    (UserInterface|Viewport|AddtoViewport _returnvalue_2 0)
    (else
      (Default|UpdateObjective _asbp_third_person_character "Gather Fuses" (Variables|/Game/ThirdPerson/Blueprints/BP_ThirdPersonCharacter.BP_ThirdPersonCharacter_C|GetFuseCount _asbp_third_person_character) 3)))
  (Actor|DestroyActor))

(event EventBeginPlay)

(event Collision|EventActorBeginOverlap
  (params (OtherActor :type Actor%20Object%20Reference)))

(event EventTick
  (params (DeltaSeconds :type Float%20%28single-precision%29)))

(fn ConstructionScript)