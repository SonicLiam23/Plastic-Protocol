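; BP_WeaponPickUp is a weapon pickup prop that hands a weapon to the character who interacts with it.
; Its Interact event calls SpawnWeapon on that character, passing the WeaponToSpawn variable and the pickup's location.
; It then plays a pickup sound at that location and destroys itself.
; Overlap and Tick are unused, so pickup happens only through Interact.
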(event EventBeginPlay
  (|CallParentFunction) ; This node is disabled and will not be called.\nDrag off pins to build functionality.
)

(event Collision|EventActorBeginOverlap
  (params (OtherActor :type Actor%20Object%20Reference))
  (|CallParentFunction OtherActor) ; This node is disabled and will not be called.\nDrag off pins to build functionality.
)

(event EventTick
  (params (DeltaSeconds :type Float%20%28single-precision%29))
  (|CallParentFunction DeltaSeconds) ; This node is disabled and will not be called.\nDrag off pins to build functionality.
)

(event EventInteract
  (params (CharacterPickingUp :type BP%20Third%20Person%20Character%20Object%20Reference))
  (bind _returnvalue (Transformation|GetActorLocation))
  (Default|SpawnWeapon CharacterPickingUp (Variables|Default|GetWeaponToSpawn) _returnvalue)
  (Audio|SpawnSoundatLocation "/Game/_Project/Audio/ammo-pickup-weapon-sound-fx_D.ammo-pickup-weapon-sound-fx_D" _returnvalue "0, 0, 0" 1.0 1.0 0.0 0 0)
  (Actor|DestroyActor))

(fn ConstructionScript
  (|CallParentFunction))